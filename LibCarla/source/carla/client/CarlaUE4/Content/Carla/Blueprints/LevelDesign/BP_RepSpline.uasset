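; Level-design spline tool that repeats a chosen static mesh along a spline as instances, built in the construction script.
; Each straight segment between points gets a capped mesh count from the spacing distance, with X scale stretched to fit exactly.
; Instances follow the segment direction or stay world-aligned, plus fixed rotation offsets and random rotation and translation.
; An optional extra mesh caps the last point, reusing the last computed rotation.
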(fn `Get the number of meshes`
  (params (MeshLenght :type "Float (double-precision)") (TotalDistance :type "Float (double-precision)"))
  (returns (Scale :type "Float (double-precision)") (`Number of Meshes` :type Integer))
  (locals (Step :type "Float (double-precision)" :default 0.0) (NewLocalVar_0 :type Integer :default 0) (NewLocalVar_1 :type "Float (double-precision)" :default 0.0) (NewLocalVar_2 :type "Float (double-precision)" :default 0.0) (`Mesh Length` :type "Float (double-precision)") (`Total Distance` :type "Float (double-precision)"))
  (bind _returnvalue (`KismetMathLibrary.FTrunc` (/ (`local.Total Distance`) (`local.Mesh Length`))))
  (bind _returnvalue_2 (* _returnvalue (`local.Mesh Length`)))
  (set `local.Mesh Length` MeshLenght)
  (set `local.Total Distance` TotalDistance)
  ;[1 1 1] Remember kids. NEVER, By any chance, allow your calculations to accidentaly divide by 0.
  (if (or (== _returnvalue_2 0.0) (== (`local.Total Distance`) 0.0))
    (return 1.0 0)
    (else
      (return (/ (`local.Total Distance`) _returnvalue_2) (- _returnvalue 1)))))

(fn `Place mesh on single point`
  (params (PointIndex :type Integer) (Target :type "InstancedStaticMeshComponent Object Reference") (TargetSpline :type "SplineComponent Object Reference"))
  (`SceneComponent.SetMobility` Target "Static")
  (`InstancedStaticMeshComponent.AddInstance` Target (`KismetMathLibrary.MakeTransform` (`SplineComponent.GetLocationAtSplinePoint` TargetSpline PointIndex "Local") (`self.MeshRotator`) (1.0 1.0 1.0))))

(fn `PlaceMeshesBetween2Points`
  (params (PointIndex :type Integer) (InstancedStaticMesh :type "InstancedStaticMeshComponent Object Reference") (Spline :type "SplineComponent Object Reference"))
  (bind _location (`SplineComponent.GetLocationAndTangentAtSplinePoint` Spline PointIndex "Local"))
  (bind (_x _y _z) (`self.RandomLocation`))
  (bind (_x_2 _y_2 _z_2) (`self.RandomRotationMacro`))
  (bind (_fixed_rotation_offset_x _fixed_rotation_offset_y _fixed_rotation_offset_z) (`self.FixedRotation`))
  (bind _distancebetweenmeshes (`self.DistanceBetweenMeshes`))
  (bind _location_2 (`SplineComponent.GetLocationAndTangentAtSplinePoint` Spline (+ PointIndex 1) "Local"))
  (bind _returnvalue (`KismetMathLibrary.FindLookAtRotation` _location _location_2))
  (bind _returnvalue_2 (+ _fixed_rotation_offset_x (+ (.roll _returnvalue) _x_2)))
  ;[1 1 1] Calculate required number of meshes for the segment
  (bind (_scale _number_of_meshes) (`self.Get the number of meshes` _distancebetweenmeshes (`KismetMathLibrary.VSize` (- _location_2 _location))))
  (for _index (range (+ (`KismetMathLibrary.Clamp` _number_of_meshes 0 (`self.MaxNumberOfMeshes`)) 1))
    ;[1 1 1] Allign vertically
    (if (`self.WorldAlignedZY`)
      (set `self.MeshRotator` (`KismetMathLibrary.MakeRotator` _returnvalue_2 (+ _y_2 _fixed_rotation_offset_y) (+ _z_2 _fixed_rotation_offset_z)))
      ;[1 1 1] AddingInstance
      (`SceneComponent.SetMobility` InstancedStaticMesh "Static")
      (else
        ;[1 1 1] Adding Offsets and Randoms
        (set `self.MeshRotator` (`KismetMathLibrary.MakeRotator` _returnvalue_2 (+ _fixed_rotation_offset_y (+ (.pitch _returnvalue) _y_2)) (+ _fixed_rotation_offset_z (+ (.yaw _returnvalue) _z_2))))))
    (`InstancedStaticMeshComponent.AddInstance` InstancedStaticMesh (`KismetMathLibrary.MakeTransform` (+ (`KismetMathLibrary.MakeVector` _x _y _z) (+ (* (* (`KismetMathLibrary.Conv_RotatorToVector` _returnvalue) _index) (* _scale _distancebetweenmeshes)) _location)) (`self.MeshRotator`) (`KismetMathLibrary.MakeVector` _scale 1.0 1.0)))))

(fn `UserConstructionScript`
  (bind _instancedstaticmesh (`self.InstancedStaticMesh`))
  ;[1 1 1] Create Static Mesh Component and Asign it
  (`StaticMeshComponent.SetStaticMesh` _instancedstaticmesh (`self.staticMesh`))
  (`PrimitiveComponent.SetCollisionEnabled` _instancedstaticmesh (`self.Collision Enabled`))
  (for _index (range (+ (- (`SplineComponent.GetNumberOfSplinePoints` (`self.Spline`)) 2) 1))
    ;[1 1 1] Place needed meshes  between in points of the spline
    (`self.PlaceMeshesBetween2Points` _index _instancedstaticmesh (`self.Spline`)))
  ;[1 1 1] Place Mesh on the last point of the spline.
  (if (`self.EndPoint`)
    (`self.Place mesh on single point` (+ _index 1) _instancedstaticmesh (`self.Spline`))))