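; WalkerFunctions is a CARLA walker helper Blueprint whose ClothingByName function restyles one named clothing material slot on a mesh.
; When the slot exists, it creates a dynamic material instance, sets tiled base color, normal, occlusion-roughness-metallic, tiling and color parameters, then assigns it to that slot.
; It always uses the first color and texture entries, since the random index picks are disconnected.
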(fn `ClothingByName`
  (params (Target :type "MeshComponent Object Reference") (`Material Slot Name` :type Name) (ColorArray :type "Array of LinearColor Structure") (TextureArray :type "Array of /Game/Carla/Static/Pedestrians/Materials/TextureStructs Structure"))
  (locals (NewLocalVar_0 :type "Array of  Structure"))
  (bind (_output_basecolor _output_normal _output_oclussionroughnessmetallic _output_tiling) (break `/Game/Carla/Static/Pedestrians/Materials/TextureStructs` (`|GetArrayItem` TextureArray)))
  (bind _returnvalue (`KismetArrayLibrary.Array_Find` (`MeshComponent.GetMaterialSlotNames` Target) `Material Slot Name`))
  (if (`MeshComponent.IsMaterialSlotNameValid` Target `Material Slot Name`)
    (bind _returnvalue_2 (`PrimitiveComponent.CreateDynamicMaterialInstance` Target _returnvalue (`|GetArrayItem` (`MeshComponent.GetMaterials` Target) _returnvalue) "None"))
    (`MaterialInstanceDynamic.SetTextureParameterValue` _returnvalue_2 "TiledTextureBaseColor" _output_basecolor)
    (`MaterialInstanceDynamic.SetTextureParameterValue` _returnvalue_2 "TiledTextureNormal" _output_normal)
    (`MaterialInstanceDynamic.SetTextureParameterValue` _returnvalue_2 "TiledTextureOclussionRoughnessMetallic" _output_oclussionroughnessmetallic)
    (`MaterialInstanceDynamic.SetScalarParameterValue` _returnvalue_2 "BasicTextureTiling" _output_tiling)
    (`MaterialInstanceDynamic.SetVectorParameterValue` _returnvalue_2 "Color" (`|GetArrayItem` ColorArray))
    (`PrimitiveComponent.SetMaterial` Target _returnvalue _returnvalue_2))
  (return))