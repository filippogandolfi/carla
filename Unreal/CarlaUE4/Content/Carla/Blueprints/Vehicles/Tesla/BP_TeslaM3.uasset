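; Player-driven CARLA Tesla Model 3 with a VR cockpit view, horn and homemade P/N/D/R gearbox.
; Tick updates km/h speed, speed-driven engine audio, and steering wheel and joystick animation, with speed and joystick behind delays.
; Gear macros toggle mutually exclusive flags to set target gear or handbrake.
; Inputs glance sideways, reset seated position, or nudge the camera only when nearly stationary; sensor-definition tests are unwired.
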(event `self.ReceiveBeginPlay`
  ;[0.6354 1 0.6498] Starting session
  (`HeadMountedDisplayFunctionLibrary.EnableHMD` true)
  (`SteamVRInputDeviceFunctionLibrary.ResetSeatedPosition` :!label _label)
  (set `self.imHere` true))

(event `Key|C`
  (params (Key :type "Key Structure"))
  ;[0.6354 1 0.6498] Starting session
  (:`Pressed`
    (goto _label)))

(event `self.ReceiveTick`
  (params (DeltaSeconds :type "Float (single-precision)"))
  (bind _returnvalue (`KismetMathLibrary.FFloor` (* (`self.GetVehicleForwardSpeed`) 0.036)))
  ;[1 0.9784 0.6302] Every tick (runtime)
  (`|ExecutionSequence`
    (:`then_0`
      (`KismetSystemLibrary.Delay` 1.0)
      (if (< _returnvalue 0)
        (set `self.vehicleVelocity` (`KismetMathLibrary.Conv_IntToDouble` (* _returnvalue -1)))
        (else
          (set `self.vehicleVelocity` (`KismetMathLibrary.Conv_IntToDouble` _returnvalue)))))
    (:`then_1`
      ;;[1 1 1] Audio
      (`AudioComponent.SetFloatParameter` (`self.Engine Sound`) "RPM" (`KismetMathLibrary.Abs` (`WheeledVehicleMovementComponent.GetForwardSpeed` (`self.VehicleMovement`)))))
    (:`then_2`
      (`SceneComponent.K2_SetRelativeRotation` (`self.steeringwheel1`) (`KismetMathLibrary.MakeRotator` -15.0 (* -100 (`self.Steering`)) 90.0) false false))
    (:`then_3`
      (`KismetSystemLibrary.Delay` 0.2)
      (`SceneComponent.K2_SetRelativeRotation` (`self.joystick2`) (`KismetMathLibrary.MakeRotator` (* 100 (`self.Steering`)) (* -100 (`self.Throttle`))) false false))))

(event `InputAction|Clacson`
  (params (Key :type "Key Structure"))
  ;[1 0.9784 0.6302] Every tick (runtime)
  ;;[1 1 1] Audio
  (:`Pressed`
    (`AudioComponent.Play` (`self.Clacson`) 0.0)))

(event `InputAction|CameraRight`
  (params (Key :type "Key Structure"))
  (bind _vrcameratm3 (`self.VRCameraTM3`))
  ;[1 0.7031 0.7031] Moving camera
  (:`Pressed`
    (`self.Vehicle is moving`)
    (`SceneComponent.K2_SetRelativeTransform` _vrcameratm3 (`KismetMathLibrary.MakeTransform` (`KismetMathLibrary.MakeVector` (.x (.location (`SceneComponent.GetRelativeTransform` _vrcameratm3))) (+ (.y (.location (`SceneComponent.GetRelativeTransform` _vrcameratm3))) 1.0) (.z (.location (`SceneComponent.GetRelativeTransform` _vrcameratm3))))) false false)))

(event `InputAction|CameraLeft`
  (params (Key :type "Key Structure"))
  (bind _vrcameratm3 (`self.VRCameraTM3`))
  ;[1 0.7031 0.7031] Moving camera
  (:`Pressed`
    (`self.Vehicle is moving`)
    (`SceneComponent.K2_SetRelativeTransform` _vrcameratm3 (`KismetMathLibrary.MakeTransform` (`KismetMathLibrary.MakeVector` (.x (.location (`SceneComponent.GetRelativeTransform` _vrcameratm3))) (+ (.y (.location (`SceneComponent.GetRelativeTransform` _vrcameratm3))) -1.0) (.z (.location (`SceneComponent.GetRelativeTransform` _vrcameratm3))))) false false)))

(event `InputAction|CameraClose`
  (params (Key :type "Key Structure"))
  ;[1 0.7031 0.7031] Moving camera
  (:`Pressed`
    (`self.Vehicle is moving`)
    (`SceneComponent.K2_SetRelativeTransform` (`self.VRCameraTM3`) (`KismetMathLibrary.MakeTransform` (`KismetMathLibrary.MakeVector` (+ (.x (.location (`SceneComponent.GetRelativeTransform` (`self.VRCameraTM3`)))) -1.0) (.y (.location (`SceneComponent.GetRelativeTransform` (`self.VRCameraTM3`)))) (.z (.location (`SceneComponent.GetRelativeTransform` (`self.VRCameraTM3`)))))) false false)))

(event `InputAction|CameraFar`
  (params (Key :type "Key Structure"))
  ;[1 0.7031 0.7031] Moving camera
  (:`Pressed`
    (`self.Vehicle is moving`)
    (`SceneComponent.K2_SetRelativeTransform` (`self.VRCameraTM3`) (`KismetMathLibrary.MakeTransform` (`KismetMathLibrary.MakeVector` (+ (.x (.location (`SceneComponent.GetRelativeTransform` (`self.VRCameraTM3`)))) 1.0) (.y (.location (`SceneComponent.GetRelativeTransform` (`self.VRCameraTM3`)))) (.z (.location (`SceneComponent.GetRelativeTransform` (`self.VRCameraTM3`)))))) false false)))

(event `InputAction|CameraUp`
  (params (Key :type "Key Structure"))
  (bind _vrcameratm3 (`self.VRCameraTM3`))
  ;[1 0.7031 0.7031] Moving camera
  (:`Pressed`
    (`self.Vehicle is moving`)
    (`SceneComponent.K2_SetRelativeTransform` _vrcameratm3 (`KismetMathLibrary.MakeTransform` (`KismetMathLibrary.MakeVector` (.x (.location (`SceneComponent.GetRelativeTransform` _vrcameratm3))) (.y (.location (`SceneComponent.GetRelativeTransform` _vrcameratm3))) (+ 1.0 (.z (.location (`SceneComponent.GetRelativeTransform` _vrcameratm3)))))) false false)))

(event `InputAction|CameraDown`
  (params (Key :type "Key Structure"))
  (bind _vrcameratm3 (`self.VRCameraTM3`))
  ;[1 0.7031 0.7031] Moving camera
  (:`Pressed`
    (`self.Vehicle is moving`)
    (`SceneComponent.K2_SetRelativeTransform` _vrcameratm3 (`KismetMathLibrary.MakeTransform` (`KismetMathLibrary.MakeVector` (.x (.location (`SceneComponent.GetRelativeTransform` _vrcameratm3))) (.y (.location (`SceneComponent.GetRelativeTransform` _vrcameratm3))) (+ (.z (.location (`SceneComponent.GetRelativeTransform` _vrcameratm3))) -1.0))) false false)))

(event `InputAction|Handbrake`
  (params (Key :type "Key Structure"))
  (bind _vehiclemovement (`self.VehicleMovement`))
  ;[0.587 0.6395 1] GearBox - HomeMade *
  (:`Pressed`
    (`|ExecutionSequence`
      (:`then_0`
        (bind _output_get (set `self.P-gear` (not (`self.P-gear`))))
        (if _output_get
          (`WheeledVehicleMovementComponent.SetHandbrakeInput` _vehiclemovement true)
          (`AudioComponent.Play` (`self.Handbrake Up`) 0.0)
          (else
            (`WheeledVehicleMovementComponent.SetHandbrakeInput` _vehiclemovement false)
            (`AudioComponent.Play` (`self.Handbrake Down`) 0.0))))
      (:`then_1`
        (set `self.D-gear` false)
        (set `self.R-gear` false)
        (set `self.N-gear` false)))))

(event `Key|One`
  (params (Key :type "Key Structure"))
  ;[0.587 0.6395 1] GearBox - HomeMade *
  (:`Pressed`
    (`|ExecutionSequence`
      (:`then_0`
        (bind _output_get (set `self.N-gear` (not (`self.N-gear`))))
        (if _output_get
          (`WheeledVehicleMovementComponent.SetTargetGear` (`self.VehicleMovement`) 0 true :!label _label_2)))
      (:`then_1`
        (set `self.D-gear` false)
        (set `self.R-gear` false)
        (set `self.P-gear` false)))))

(event `Key|Two`
  (params (Key :type "Key Structure"))
  ;[0.587 0.6395 1] GearBox - HomeMade *
  (:`Pressed`
    (`|ExecutionSequence`
      (:`then_0`
        (bind _output_get (set `self.D-gear` (not (`self.D-gear`))))
        (if _output_get
          (`WheeledVehicleMovementComponent.SetTargetGear` (`self.VehicleMovement`) 1 true)
          (else
            (goto _label_2))))
      (:`then_1`
        (set `self.P-gear` false)
        (set `self.R-gear` false)
        (set `self.N-gear` false)))))

(event `Key|Three`
  (params (Key :type "Key Structure"))
  ;[0.587 0.6395 1] GearBox - HomeMade *
  (:`Pressed`
    (`|ExecutionSequence`
      (:`then_0`
        (bind _output_get (set `self.R-gear` (not (`self.R-gear`))))
        (if _output_get
          (`WheeledVehicleMovementComponent.SetTargetGear` (`self.VehicleMovement`) -1 true)
          (else
            (goto _label_2))))
      (:`then_1`
        (set `self.D-gear` false)
        (set `self.N-gear` false)
        (set `self.P-gear` false)))))

(event `self.ReceiveActorBeginOverlap`
  (params (OtherActor :type "Actor Object Reference"))
  (`parent.ReceiveActorBeginOverlap` OtherActor))

(event `InputAction|LookLeft`
  (params (Key :type "Key Structure"))
  ;[0.7292 1 0.9781] Rotate view for corners
  ;;[1 1 1 1 9] It could be possible to substitute keyboard with trigger
  (:`Pressed`
    (`SceneComponent.K2_SetRelativeRotation` (`self.VRCameraTM3`) (`KismetMathLibrary.MakeRotator` 0.0 0.0 (`self.look around`)) false false))
  (:`Released`
    (`SceneComponent.K2_SetRelativeRotation` (`self.VRCameraTM3`) (`KismetMathLibrary.MakeRotator` 0.0) false false)))

(event `InputAction|LookRight`
  (params (Key :type "Key Structure"))
  ;[0.7292 1 0.9781] Rotate view for corners
  (:`Pressed`
    (`SceneComponent.K2_SetRelativeRotation` (`self.VRCameraTM3`) (`KismetMathLibrary.MakeRotator` 0.0 0.0 (* (`self.look around`) -1.0)) false false))
  (:`Released`
    (`SceneComponent.K2_SetRelativeRotation` (`self.VRCameraTM3`) (`KismetMathLibrary.MakeRotator` 0.0) false false)))

(fn `SetTimer`
  (set `self.Timer` (- (`self.Timer`) 1)))

(fn `UserConstructionScript`
  (`parent.UserConstructionScript`))

(fn `Vehicle is moving`
  (if (!= (`KismetMathLibrary.FFloor` (* (`self.GetVehicleForwardSpeed`) 0.036)) 0)
    (`KismetSystemLibrary.PrintString` "wait")
    (else
      (return))))