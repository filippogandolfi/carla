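; Traffic light Blueprint for CARLA that builds its signal heads and props and shows the current light state.
; The construction script spawns support and lens meshes from Heads, giving each lens a masked or master dynamic material, tinted and sorted into red, yellow and green arrays.
; State changes toggle the "On/Off" scalar on those arrays.
; BoxTrigger overlaps by CARLA wheeled vehicles call NotifyWheeledVehicle, and GetTriggerVolume exposes that box.
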(event `self.OnTrafficLightStateChanged`
  (params (TrafficLightState :type "ETrafficLightState Enum" :default "Red"))
  (switch `ETrafficLightState` TrafficLightState
    (:`Red`
      (for _array_element (`self.RedLights`)
        (`MaterialInstanceDynamic.SetScalarParameterValue` _array_element "On/Off" 1.0))
      (for _array_element_2 (`self.YellowLights`)
        (`MaterialInstanceDynamic.SetScalarParameterValue` _array_element_2 "On/Off" 0.0))
      (for _array_element_3 (`self.GreenLights`)
        (`MaterialInstanceDynamic.SetScalarParameterValue` _array_element_3 "On/Off" 0.0)))
    (:`Yellow`
      (for _array_element_4 (`self.RedLights`)
        (`MaterialInstanceDynamic.SetScalarParameterValue` _array_element_4 "On/Off" 0.0))
      (for _array_element_5 (`self.YellowLights`)
        (`MaterialInstanceDynamic.SetScalarParameterValue` _array_element_5 "On/Off" 1.0))
      (for _array_element_6 (`self.GreenLights`)
        (`MaterialInstanceDynamic.SetScalarParameterValue` _array_element_6 "On/Off" 0.0)))
    (:`Green`
      (for _array_element_7 (`self.RedLights`)
        (`MaterialInstanceDynamic.SetScalarParameterValue` _array_element_7 "On/Off" 0.0))
      (for _array_element_8 (`self.YellowLights`)
        (`MaterialInstanceDynamic.SetScalarParameterValue` _array_element_8 "On/Off" 0.0))
      (for _array_element_9 (`self.GreenLights`)
        (`MaterialInstanceDynamic.SetScalarParameterValue` _array_element_9 "On/Off" 1.0)))))

(event `self.BoxTrigger.OnComponentBeginOverlap`
  (params (OverlappedComponent :type "PrimitiveComponent Object Reference") (OtherActor :type "Actor Object Reference") (OtherComp :type "PrimitiveComponent Object Reference") (OtherBodyIndex :type Integer) (bFromSweep :type Boolean) (SweepResult :type "HitResult Structure (by ref)"))
  (bind _ascarla_wheeled_vehicle (cast `CarlaWheeledVehicle` OtherActor))
  (`self.NotifyWheeledVehicle` _ascarla_wheeled_vehicle))

(event `self.BoxTrigger.OnComponentEndOverlap`
  (params (OverlappedComponent :type "PrimitiveComponent Object Reference") (OtherActor :type "Actor Object Reference") (OtherComp :type "PrimitiveComponent Object Reference") (OtherBodyIndex :type Integer)))

(fn `GetTriggerVolume`
  (returns (ReturnValue :type "BoxComponent Object Reference"))
  (return (`self.BoxTrigger`)))

(fn `UserConstructionScript`
  (locals (CurrentMaterial :type "MaterialInstanceDynamic Object Reference"))
  (bind _currentmaterial (`local.CurrentMaterial`))
  (bind _currentmaterial_2 (`local.CurrentMaterial`))
  (`|ExecutionSequence`
    (:`then_0`
      (for _array_element (`self.Heads`)
        (bind (_description _position _lights _support) (break `/Game/Carla/Blueprints/TrafficLight/ST_TrafficLightHead` _array_element))
        (bind _returnvalue (`AddComponent|NODE_AddStaticMeshComponent-1` :`RelativeTransform` _position))
        (`StaticMeshComponent.SetStaticMesh` _returnvalue _support)
        (for _array_element_2 _lights
          (bind (_mesh _relativetransform _lightcolor _masked _mask _rotation) (break `/Game/Carla/Static/TrafficSigns/Streetlights_01/TrafficLightPieceStructure` _array_element_2))
          (bind _returnvalue_2 (`AddComponent|NODE_AddStaticMeshComponent-2` :`RelativeTransform` _relativetransform))
          (`SceneComponent.K2_AttachToComponent` _returnvalue_2 _returnvalue "None" "KeepRelative" "KeepRelative" "KeepRelative" false)
          (`StaticMeshComponent.SetStaticMesh` _returnvalue_2 _mesh)
          (if _masked
            (bind _returnvalue_3 (`PrimitiveComponent.CreateDynamicMaterialInstance` _returnvalue_2 1 "/Game/Carla/Static/TrafficSigns/TrafficLight/M_StreetlightsMasked_T10.M_StreetlightsMasked_T10" "None"))
            (set `local.CurrentMaterial` _returnvalue_3)
            (else
              (bind _returnvalue_4 (`PrimitiveComponent.CreateDynamicMaterialInstance` _returnvalue_2 1 "/Game/Carla/Static/TrafficSigns/TrafficLight/M_StreetlightsMaster_T10.M_StreetlightsMaster_T10" "None"))
              (set `local.CurrentMaterial` _returnvalue_4)))
          (`MaterialInstanceDynamic.SetTextureParameterValue` _currentmaterial_2 "LightMask" _mask)
          (`MaterialInstanceDynamic.SetScalarParameterValue` _currentmaterial_2 "Angle" _rotation)
          (switch `/Game/Carla/Static/TrafficSigns/Streetlights_01/StreetLightColor` _lightcolor
            (:`NewEnumerator0`
              (`MaterialInstanceDynamic.SetVectorParameterValue` _currentmaterial "LightColor" (struct :`R` 1.0 :`G` 0.015686 :`A` 1.0))
              (`KismetArrayLibrary.Array_Add` (`self.RedLights`) _currentmaterial))
            (:`NewEnumerator1`
              (`MaterialInstanceDynamic.SetVectorParameterValue` _currentmaterial "LightColor" (struct :`R` 1.0 :`G` 0.745098 :`A` 1.0))
              (`KismetArrayLibrary.Array_Add` (`self.YellowLights`) _currentmaterial))
            (:`NewEnumerator2`
              (`MaterialInstanceDynamic.SetVectorParameterValue` _currentmaterial "LightColor" (struct :`G` 1.0 :`A` 1.0))
              (`KismetArrayLibrary.Array_Add` (`self.GreenLights`) _currentmaterial))))))
    (:`then_1`
      (for _array_element_3 (`self.Props`)
        (bind (_prop _rotation_2 _heigh) (break `/Game/Carla/Blueprints/TrafficLight/ST_TrafficLightProps` _array_element_3))
        (`/Engine/EditorBlueprintResources/StandardMacros.IsValid` _prop
          (:`Is Valid`
            (bind _returnvalue_5 (`AddComponent|NODE_AddStaticMeshComponent-4` :`RelativeTransform` (`KismetMathLibrary.MakeTransform` (`KismetMathLibrary.MakeVector` 0.0 0.0 _heigh) (`KismetMathLibrary.MakeRotator` 0.0 0.0 _rotation_2))))
            (`StaticMeshComponent.SetStaticMesh` _returnvalue_5 _prop)))))))