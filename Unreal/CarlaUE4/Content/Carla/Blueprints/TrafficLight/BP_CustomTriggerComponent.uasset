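; Trigger component for BP_TrafficLightNew that holds a single CARLA wheeled vehicle at a non-green light.
; BeginPlay caches the owning traffic light, and BindOverlap hooks the box collider's begin-overlap event.
; An overlapping vehicle is stored as the stopped car and passed to the light's notify call, unless one is already held.
; When LightTrafficStateChanged reports green, the component un-notifies that vehicle and clears it.
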(event `self.ReceiveBeginPlay`
  (bind _asbp_traffic_light_new (cast `/Game/Carla/Static/TrafficSigns/Streetlights_01/BP_TrafficLightNew` (`self.GetOwner`)))
  (set `self.TrafficLight` _asbp_traffic_light_new))

(event `BindOverlap`
  (add `PrimitiveComponent.OnComponentBeginOverlap` (`self.BoxCollider`) (delegate `OnComponentBeginOverlap`)))

(event `OnComponentBeginOverlap`
  (params (OverlappedComponent :type "PrimitiveComponent Object Reference") (OtherActor :type "Actor Object Reference") (OtherComp :type "PrimitiveComponent Object Reference") (OtherBodyIndex :type Integer) (bFromSweep :type Boolean) (SweepResult :type "HitResult Structure (by ref)"))
  (`/Engine/EditorBlueprintResources/StandardMacros.IsValid` (`self.TrafficLight`)
    (:`Is Valid`
      (if (`|EnumInequality` (`TrafficLightBase.GetTrafficLightState` (`self.TrafficLight`)) "Green")
        (`/Engine/EditorBlueprintResources/StandardMacros.IsValid` (`self.StoppedCar`)
          (:`Is Not Valid`
            (bind _ascarla_wheeled_vehicle (cast `CarlaWheeledVehicle` OtherActor))
            (bind _output_get (set `self.StoppedCar` _ascarla_wheeled_vehicle))
            (`TrafficLightBase.NotifyWheeledVehicle` (`self.TrafficLight`) _output_get)))))))

(event `LightTrafficStateChanged`
  (params (LightState :type "ETrafficLightState Enum" :default "Red"))
  (bind _stoppedcar (`self.StoppedCar`))
  (if (== (enumliteral `ETrafficLightState` "Green") LightState)
    (`/Engine/EditorBlueprintResources/StandardMacros.IsValid` _stoppedcar
      (:`Is Valid`
        (`TrafficLightBase.UnNotifyWheeledVehicle` (`self.TrafficLight`) _stoppedcar)
        (set `self.StoppedCar` null)))))